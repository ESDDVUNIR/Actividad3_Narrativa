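; Player character Blueprint with Enhanced Input movement, look, jump, a walk/run speed toggle and camera-based interaction.
; Moving on the ground starts a looping footstep timer, cleared when move input completes, and landing from a fall plays a step.
; Interact line-traces from the camera and sends InteractMessage to the hit actor.
; Q toggles a spotlight with a switch sound, playing an extra sound the first time it turns on.
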(event `self.ReceiveBeginPlay`
  ;[1 1 1] Set controller
  (`|ExecutionSequence`
    (:`then_0`
      (bind _asplayer_controller (cast `PlayerController` (`self.GetController`)))
      (bind _returnvalue (pcsubsystem `EnhancedInputLocalPlayerSubsystem` _asplayer_controller))
      (`/Engine/EditorBlueprintResources/StandardMacros.IsValid` _returnvalue
        (:`Is Valid`
          (`EnhancedInputSubsystemInterface.AddMappingContext` _returnvalue "/Game/Input/IMC_Default.IMC_Default" 0 (struct)))))))

(event `EnhancedInput|/Game/Input/Actions/IA_LookUp`
  (params (ActionValue :type "Float (double-precision)") (ElapsedSeconds :type "Float (double-precision)") (TriggeredSeconds :type "Float (double-precision)") (InputAction :type "InputAction Object Reference" :default "/Game/Input/Actions/IA_LookUp.IA_LookUp"))
  ;[1 1 1] Look
  (:`Triggered`
    (`self.AddControllerPitchInput` (* ActionValue 0.5))))

(event `EnhancedInput|/Game/Input/Actions/IA_Turn`
  (params (ActionValue :type "Float (double-precision)") (ElapsedSeconds :type "Float (double-precision)") (TriggeredSeconds :type "Float (double-precision)") (InputAction :type "InputAction Object Reference" :default "/Game/Input/Actions/IA_Turn.IA_Turn"))
  ;[1 1 1] Look
  (:`Triggered`
    (`self.AddControllerYawInput` (* ActionValue 0.5))))

(event `EnhancedInput|/Game/Input/Actions/IA_Move`
  (params (ActionValue :type "Vector2D Structure") (ElapsedSeconds :type "Float (double-precision)") (TriggeredSeconds :type "Float (double-precision)") (InputAction :type "InputAction Object Reference" :default "/Game/Input/Actions/IA_Move.IA_Move"))
  (bind (_returnvalue_roll _returnvalue_pitch _returnvalue_yaw) (`KismetMathLibrary.BreakRotator` (`self.GetControlRotation`)))
  (bind (_returnvalue_x _returnvalue_y _returnvalue_z) (`KismetMathLibrary.BreakVector` (`self.GetVelocity`)))
  (bind (_returnvalue_roll_2 _returnvalue_pitch_2 _returnvalue_yaw_2) (`KismetMathLibrary.BreakRotator` (`self.GetControlRotation`)))
  ;[1 1 1] Move
  (:`Triggered`
    (`self.AddMovementInput` (`KismetMathLibrary.GetRightVector` (`KismetMathLibrary.MakeRotator` _returnvalue_roll 0.0 _returnvalue_yaw)) ActionValue_X)
    (`self.AddMovementInput` (`KismetMathLibrary.GetForwardVector` (`KismetMathLibrary.MakeRotator` _returnvalue_roll_2 0.0 _returnvalue_yaw_2)) ActionValue_Y)
    ;[1 1 1] Footsteps SFX
    (if (and (or (> _returnvalue_x 2.0) (< _returnvalue_x -2.0) (> _returnvalue_y 2.0) (< _returnvalue_y -2.0)) (== _returnvalue_z 0.0))
      (`/Engine/EditorBlueprintResources/StandardMacros.DoOnce` false :!label _label
        (:`Completed`
          (bind _returnvalue (`KismetSystemLibrary.K2_SetTimerDelegate` (delegate `PlayFootStepSound`) (`self.FootStep Interval`) true))))))
  (:`Completed`
    (`KismetSystemLibrary.K2_ClearAndInvalidateTimerHandle` _returnvalue)
    (goto _label :!via `Reset`)))

(event `PlayFootStepSound`
  ;[1 1 1] Footsteps SFX
  (`GameplayStatics.PlaySoundAtLocation` "/Game/Sounds/Steps.Steps" (- (`self.K2_GetActorLocation`) (0.0 0.0 44.0)) (struct) 4.0 1.0 0.0 null null null null))

(event `EnhancedInput|/Game/Input/Actions/IA_Jump`
  (params (ActionValue :type Boolean) (ElapsedSeconds :type "Float (double-precision)") (TriggeredSeconds :type "Float (double-precision)") (InputAction :type "InputAction Object Reference" :default "/Game/Input/Actions/IA_Jump.IA_Jump"))
  ;[1 1 1] Interact
  (:`Triggered`
    (`self.Jump`)))

(event `EnhancedInput|/Game/Input/Actions/IA_Run`
  (params (ActionValue :type Boolean) (ElapsedSeconds :type "Float (double-precision)") (TriggeredSeconds :type "Float (double-precision)") (InputAction :type "InputAction Object Reference" :default "/Game/Input/Actions/IA_Run.IA_Run"))
  (bind _charactermovement (`self.CharacterMovement`))
  ;[1 1 1] Correr
  (:`Started`
    (`/Engine/EditorBlueprintResources/StandardMacros.FlipFlop`
      (:`A`
        (set `CharacterMovementComponent.MaxWalkSpeed` 600.0 _charactermovement))
      (:`B`
        (set `CharacterMovementComponent.MaxWalkSpeed` 300.0 _charactermovement)))))

(event `self.K2_OnMovementModeChanged`
  (params (PrevMovementMode :type "EMovementMode Enum" :default "MOVE_None") (NewMovementMode :type "EMovementMode Enum" :default "MOVE_None") (PrevCustomMode :type Byte) (NewCustomMode :type Byte))
  ;[1 1 1] Footsteps SFX
  (if (and (`|EnumEquality` PrevMovementMode "MOVE_Falling") (`|EnumEquality` NewMovementMode "MOVE_Walking"))
    (`self.PlayFootStepSound`)))

(event `EnhancedInput|/Game/Input/Actions/IA_Interact`
  (params (ActionValue :type Boolean) (ElapsedSeconds :type "Float (double-precision)") (TriggeredSeconds :type "Float (double-precision)") (InputAction :type "InputAction Object Reference" :default "/Game/Input/Actions/IA_Interact.IA_Interact"))
  (bind _camera (`self.Camera`))
  (bind _returnvalue (`SceneComponent.K2_GetComponentLocation` _camera))
  ;[1 1 1] Interaction
  (:`Started`
    (bind (_outhit _returnvalue_2) (`KismetSystemLibrary.LineTraceSingle` _returnvalue (+ (* (`KismetMathLibrary.GetForwardVector` (`SceneComponent.K2_GetComponentRotation` _camera)) 1000.0) _returnvalue) "TraceTypeQuery1"))
    (if _returnvalue_2
      (message `/Game/Interface/Interact_Interface.Interact` (`.HitActor` (`GameplayStatics.BreakHitResult` _outhit))))))

(event `Key|Q`
  (params (Key :type "Key Structure"))
  (bind _spotlight (`self.SpotLight`))
  ;[1 1 1] Lampara On off
  (:`Pressed`
    (`/Engine/EditorBlueprintResources/StandardMacros.FlipFlop`
      (:`A`
        (`GameplayStatics.PlaySound2D` "/Game/Sounds/switch.switch" 1.0 1.0 0.0 null null)
        (`LightComponent.SetIntensity` _spotlight 500.0)
        (`/Engine/EditorBlueprintResources/StandardMacros.DoOnce` false
          (:`Completed`
            (`GameplayStatics.PlaySound2D` "/Game/Sounds/TXT05.TXT05" 10.0 1.0 0.0 null null))))
      (:`B`
        (`GameplayStatics.PlaySound2D` "/Game/Sounds/switch.switch" 1.0 1.0 0.0 null null)
        (`LightComponent.SetIntensity` _spotlight 0.0)))))

(fn `UserConstructionScript`)